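; BP_CLBufferTest is a sandbox test Blueprint for running a compute kernel (likely OpenCL) on a float buffer.
; On BeginPlay it creates the buffer and program from its variables, passing an integer and the buffer as kernel arguments.
; It runs the kernel in one dimension across the array's length, then reads the buffer back and prints each element, or prints a failure message.
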(event `self.ReceiveBeginPlay`
  (bind _buffer (`self.Buffer`))
  (bind _returnvalue (`KismetArrayLibrary.Array_Length` _buffer))
  (bind _returnvalue_2 (`CLWorksLibrary.CreateFloatBuffer` _buffer "READ_WRITE" "STREAM" null))
  (bind _returnvalue_3 (`CLWorksLibrary.CreateProgram` (`self.Program`) (`self.ProgramName`) null))
  (`CLProgramObject.SetIntArg` _returnvalue_3 0 (`self.Mod_Integer`))
  (`CLProgramObject.SetBufferArg` _returnvalue_3 1 _returnvalue_2)
  (bind _returnvalue_4 (`CLWorksLibrary.RunProgram` _returnvalue_3 1 (`|MakeArray` (`KismetMathLibrary.Conv_IntToInt64` _returnvalue)) null))
  (if _returnvalue_4
    (bind _returnvalue_5 (`CLWorksLibrary.ReadFloatBuffer` _returnvalue_2 _returnvalue null null))
    (`KismetSystemLibrary.PrintString` "Buffer Results:")
    (for _array_element _returnvalue_5
      (`KismetSystemLibrary.PrintString` (`KismetStringLibrary.Conv_DoubleToString` _array_element)))
    (else
      (`KismetSystemLibrary.PrintString` "Failed Program!"))))

(fn `UserConstructionScript`)